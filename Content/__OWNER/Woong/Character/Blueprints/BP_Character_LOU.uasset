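; Top-down character Blueprint for LOU that casts a mouse-aimed skill on the Q key.
; Tick snaps a world cursor component to the surface hit under the mouse, aligned to its normal.
; Q stores a yaw-only look-at rotation toward that cursor, turns the character and spawns BP_SkillA2 at the SkillArrowPoint.
; After a short delay it fires a second shot, reapplying the saved rotation rather than re-aiming.
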(event `Key|Q`
  (params (Key :type "Key Structure"))
  (:`Pressed`
    ;[1 1 1] 액터와 마우스 사이의 회전값 저장
    (`self.FindActorMouseRotation`)
    ;[1 1 1] 액터를 마우스 포인터의 방향으로 턴
    (`self.TurnActor`)
    ;[1 1 1] 액터 스폰
    (`self.SpawnSkillA`)
    ;[1 1 1] 한번 더 실행
    (`KismetSystemLibrary.Delay` 0.2)
    (`self.TurnActor`)
    (`self.SpawnSkillA`)))

(event `self.ReceiveTick`
  (params (DeltaSeconds :type "Float (single-precision)"))
  (bind (_bblockinghit _binitialoverlap _time _distance _location _impactpoint _normal _impactnormal) (`GameplayStatics.BreakHitResult` (`PlayerController.GetHitResultUnderCursorByChannel` (`GameplayStatics.GetPlayerController` 0) "TraceTypeQuery1" true)))
  ;[1 1 1] 매 프레임 커서의 트랜스폼을 설정
  (`SceneComponent.K2_SetWorldLocationAndRotation` (`self.CursorToWorld`) _location (`KismetMathLibrary.MakeRotationFromAxes` _impactnormal) false false))

(fn `FindActorMouseRotation`
  (bind (_returnvalue_x _returnvalue_y _returnvalue_z) (`KismetMathLibrary.BreakVector` (`self.K2_GetActorLocation`)))
  (bind (_returnvalue_x_2 _returnvalue_y_2) (`KismetMathLibrary.BreakVector` (`SceneComponent.K2_GetComponentLocation` (`self.CursorToWorld`))))
  (set `self.FindRotation` (`KismetMathLibrary.FindLookAtRotation` (`KismetMathLibrary.MakeVector` _returnvalue_x _returnvalue_y _returnvalue_z) (`KismetMathLibrary.MakeVector` _returnvalue_x_2 _returnvalue_y_2 _returnvalue_z))))

(fn `SpawnSkillA`
  (bind (_returnvalue_location _returnvalue_rotation _returnvalue_scale) (`KismetMathLibrary.BreakTransform` (`self.GetTransform`)))
  (`|SpawnActorFromClass` "/Game/__OWNER/Woong/Blueprints/BP_SkillA2.BP_SkillA2_C" (`KismetMathLibrary.MakeTransform` (`SceneComponent.K2_GetComponentLocation` (`self.SkillArrowPoint`)) _returnvalue_rotation _returnvalue_scale) "Undefined" "OverrideRootScale" null null))

(fn `TurnActor`
  (`self.K2_SetActorRelativeRotation` (`self.FindRotation`)))

(fn `UserConstructionScript`)